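; BP_Carrot is a carrot pickup that players pull from grow beds and carry, with a win check on pickup.
; On BeginPlay it links to an overlapping BP_GrowBed and disables that bed's trigger.
; Interact attaches it to an empty-handed character's CarrotSocket, notifies BPCarrotComponent and frees the bed.
; If the carrot has reached its target scale, it prints the winning player's color from the controller ID.
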(event EventInteract
  (params (bHasCarrot :type Boolean) (Character :type BP%20Top%20Down%20Character%20Object%20Reference))
  (bind _bp_carrotcomponent (Variables|Default|GetBP_CarrotComponent))
  (if (not bHasCarrot)
    (Utilities|FlowControl|Sequence
      (:then_0
        (Default|CarrotNotinBed (Variables|Default|GetBP_CarrotComponent))
        (Transformation|AttachComponentToComponent (Variables|/Script/Engine.Character|GetMesh Character) "CarrotSocket" "KeepRelative" "KeepRelative" "KeepRelative" true)
        (Transformation|SetActorRelativeLocation "0, 0, 0")
        (Variables|/Game/TopDown/Blueprints/BP_TopDownCharacter.BP_TopDownCharacter_C|SetCarrot Character self)
        (Collision|SetCollisionEnabled (Variables|Default|GetTrigger) "NoCollision")
        (Utilities|IsValid (Variables|Default|GetGrowBed)
          (:Is%20Valid
            (Collision|SetCollisionEnabled (Variables|/Game/Blueprints/Environment/BP_GrowBed.BP_GrowBed_C|GetTrigger (Variables|Default|GetGrowBed)) "QueryOnly")
            (Variables|Default|SetGrowBed 0))))
      (:then_1
        (if (>= (Variables|/Game/Blueprints/Items/BP_CarrotComponent.BP_CarrotComponent_C|GetCarrotScale _bp_carrotcomponent) (Variables|/Game/Blueprints/Items/BP_CarrotComponent.BP_CarrotComponent_C|GetTargetCarrotScale _bp_carrotcomponent))
          (bind _asbp_twin_stick_controller (Utilities|Casting|CastToBP_TwinStickController (Pawn|GetController Character)))
          (Development|PrintString (Utilities|String|Append "Winning Player:  " (Utilities|Select :Index (Class|GameplayStatics|GetPlayerControllerID _asbp_twin_stick_controller) :Option%200 "Red" :Option%201 "Blue" :Option%202 "Green" :Option%203 "Yellow"))))))))

(event EventBeginPlay
  (bind _array_element (Utilities|Array|ForEachLoopwithBreak (Collision|GetOverlappingActors 0 :!class /Script/Engine.Actor) :!label _label)
    (:LoopBody
      (bind _asbp_grow_bed (Utilities|Casting|CastToBP_GrowBed _array_element))
      (bind _output_get (Variables|Default|SetGrowBed _asbp_grow_bed))
      (Collision|SetCollisionEnabled (Variables|/Game/Blueprints/Environment/BP_GrowBed.BP_GrowBed_C|GetTrigger _output_get) "NoCollision")
      (goto _label Break))))

(fn ConstructionScript)