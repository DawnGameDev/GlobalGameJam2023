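; Actor component that makes a carrot grow over time by scaling the owner's static mesh.
; On BeginPlay it caches the mesh, applies the initial scale and starts a looping timer that adds a growth increment until the target scale is reached.
; CarrotNotInBed clears that timer, and CarrotInBed starts it.
; Every scale change also writes the value to CarrotPercent on the BP_TwinStickGameMode UI.
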(event Custom|CarrotInBed
  (bind _carrotgrowthtimer (Variables|Default|GetCarrotGrowthTimer))
  (bind _returnvalue (Utilities|Time|SetTimerbyEvent (delegate Custom|IncreaseCarrotScale) _carrotgrowthtimer true _carrotgrowthtimer)))

(event Custom|CarrotNotInBed
  (Utilities|Time|ClearandInvalidateTimerbyHandle (stale Custom|CarrotInBed _returnvalue)))

(event Custom|IncreaseCarrotScale
  (CallFunction|SetCarrotScale (+ (Variables|Default|GetCarrotScale) (Variables|Default|GetCarrotGrowthRate)))
  (if (>= (Variables|Default|GetCarrotScale) (Variables|Default|GetTargetCarrotScale))
    (Utilities|Time|ClearandInvalidateTimerbyHandle (stale Custom|CarrotInBed _returnvalue))))

(event EventBeginPlay
  (Variables|Default|SetStaticMesh (Actor|GetComponentbyClass (Components|GetOwner) "/Script/Engine.StaticMeshComponent"))
  (CallFunction|SetCarrotScale (Variables|Default|GetInitialCarrotScale))
  (CallFunction|CarrotinBed))

(fn SetCarrotScale
  (params (Scale :type Float%20%28double-precision%29))
  (bind _output_get (Variables|Default|SetCarrotScale Scale))
  (CallFunction|SetMeshScale (Variables|Default|GetStaticMesh) (Math|Vector|MakeVector _output_get _output_get _output_get))
  (bind _asbp_twin_stick_game_mode (Utilities|Casting|CastToBP_TwinStickGameMode (Game|GetGameMode)))
  (Variables|/Game/UI/GameUI.GameUI_C|SetCarrot%20Percent (Variables|/Game/Blueprints/GameModes/BP_TwinStickGameMode.BP_TwinStickGameMode_C|GetUi _asbp_twin_stick_game_mode) (Variables|Default|GetCarrotScale)))

(fn SetMeshScale
  (params (Mesh :type Mesh%20Component%20Object%20Reference) (Scale :type Vector))
  (Utilities|IsValid Mesh
    (:Is%20Valid
      (Transformation|SetRelativeScale3D Mesh Scale))))