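; Health component that tracks an actor's health and kills an owning BP_TopDownCharacter when health runs out.
; SubtractHealth and AddHealth clamp the value between zero and MaxHealth, with SubtractHealth calling Die on the character at zero.
; OnDamaged plays a hit sound and restarts a delayed looping timer that regenerates health through AddHealth until it is full.
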(event Custom|OnDamaged
  (Utilities|Time|ClearTimerbyFunctionName 0 "RegenHealth")
  (Utilities|Time|SetTimerbyFunctionName 0 "RegenHealth" 1.0 true 5.0)
  (Audio|PlaySoundatLocation "/Game/Sound_Assets/take_dmg.take_dmg" (Transformation|GetActorLocation (Components|GetOwner)) "0, 0, 0" 3.0 1.0 0.0 0 0 0 0))

(event EventBeginPlay
  (Variables|Default|SetHealth (Variables|Default|GetMaxHealth)))

(fn SubtractHealth
  (params (Amount :type Float%20%28double-precision%29))
  (Variables|Default|SetHealth (- (Variables|Default|GetHealth) Amount))
  (if (<= (Variables|Default|GetHealth) 0.0)
    (Variables|Default|SetHealth 0.0)
    (bind _asbp_top_down_character (Utilities|Casting|CastToBP_TopDownCharacter (Components|GetOwner)))
    (Default|Die _asbp_top_down_character)))

(fn AddHealth
  (params (Amount :type Float%20%28double-precision%29))
  (Variables|Default|SetHealth (+ (Variables|Default|GetHealth) Amount))
  (if (>= (Variables|Default|GetHealth) (Variables|Default|GetMaxHealth))
    (Variables|Default|SetHealth (Variables|Default|GetMaxHealth))
    (Utilities|Time|ClearTimerbyFunctionName 0 "RegenHealth")))

(fn RegenHealth
  (CallFunction|AddHealth (Variables|Default|GetHealthRegenAmount)))